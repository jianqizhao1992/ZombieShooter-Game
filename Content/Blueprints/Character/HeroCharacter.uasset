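; Player hero character Blueprint that toggles between a high camera showing the body mesh and a low camera showing first-person meshes.
; BeginPlay creates the status widget and starts with the body mesh visible and the first-person mesh and gun location hidden.
; ToggleCamera switches cameras, restores game-only input and calls SwitchGun, then sets body and first-person mesh visibility from HighCameraActive, propagating to child components.
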(event `self.ReceiveBeginPlay`
  (bind _returnvalue (`|CreateWidget` "/Game/Blueprints/Mode/StatusWidget.StatusWidget_C"))
  (`UserWidget.AddToViewport` _returnvalue 0)
  (`SceneComponent.SetVisibility` (`self.Mesh`) true true)
  (`SceneComponent.SetVisibility` (`self.MeshFirstPerson`) false true)
  (`SceneComponent.SetVisibility` (`self.GunTempLocFirstPerson`) false true))

(event `self.ToggleCamera`
  (`self.SwitchCamera` (`self.CameraHigh`) (`self.CameraLow`))
  (`WidgetBlueprintLibrary.SetInputMode_GameOnly` (`GameplayStatics.GetPlayerController` 0))
  (`self.SwitchGun`)
  (if (`self.HighCameraActive`)
    (`SceneComponent.SetVisibility` (`self.Mesh`) true true)
    (`SceneComponent.SetVisibility` (`self.MeshFirstPerson`) false true)
    (else
      (`SceneComponent.SetVisibility` (`self.Mesh`) false true)
      (`SceneComponent.SetVisibility` (`self.MeshFirstPerson`) true true))))

(fn `UserConstructionScript`)